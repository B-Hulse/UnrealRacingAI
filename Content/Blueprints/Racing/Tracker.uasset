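; Race manager that runs a race from start screen and countdown through laps to the Time Trial or Head-to-Head end screen.
; Numbered checkpoints report activations, which advance racers only in sequence, update reset points and detect finishes.
; A looping timer ranks Head-to-Head racers live by laps, checkpoints and fractional segment distance, with final positions ordered by total time.
; A timeline serves as the race clock, feeding HUD text.
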(event Custom|RaceFinished
  ;[1 1 1] Race finished
  (Variables|Default|SetRaceState "NewEnumerator2")
  (CallFunction|StopRaceTime)
  (Utilities|Time|ClearandInvalidateTimerbyHandle (Variables|Default|GetUpdatePositionsHandle))
  (Variables|DisplayText|SetDisplayedFinalRaceTime (Utilities|TimetoText (.TotalTime (Utilities|Struct|BreakRacerData (Utilities|Array|Get(acopy) (Variables|RacerData|GetRacers) (Variables|RacerData|GetDisplayedRacerID))))))
  (switch Utilities|FlowControl|Switch|SwitchonRaceMode (Variables|Default|GetTrackerMode)
    (:NewEnumerator0
      ;;[1 1 1] Time Trail: Show Final Time on HUD
      (Default|ShowTTEndScreen (Variables|References|GetHUDRef))
      (Default|CallRaceEnd))
    (:NewEnumerator1
      ;;[1 1 1] Head-to-Head: Assign Final positions to racers, display winner on HUD
      (CallFunction|AssignPositions true)
      (bind _array_element (Utilities|Array|ForEachLoopwithBreak (Variables|RacerData|GetRacers))
        (:LoopBody
          (if (== (.Position (Utilities|Struct|BreakRacerData _array_element)) 1)
            (Default|ShowH2HEndScreen (Variables|References|GetHUDRef) (.RacerID (Utilities|Struct|BreakRacerData _array_element)))
            (Default|CallRaceEnd)))))))

(event Custom|CountdownStart
  ;[1 1 1] Countdown and Race Initiation
  (Default|ShowCountdown (Variables|References|GetHUDRef))
  (Variables|Default|SetRaceState "NewEnumerator3")
  (Variables|DisplayText|SetCountdownText "3")
  (Utilities|FlowControl|Delay 1.0)
  (Variables|DisplayText|SetCountdownText "2")
  (Utilities|FlowControl|Delay 1.0)
  (Variables|DisplayText|SetCountdownText "1")
  (Utilities|FlowControl|Delay 1.0)
  (Variables|DisplayText|SetCountdownText "Go!")
  (Default|CallRaceStart)
  (CallFunction|StartRaceTime)
  (Variables|Default|SetRaceState "NewEnumerator1")
  (Utilities|FlowControl|Delay 1.0)
  (Default|ShowIngame (Variables|References|GetHUDRef)))

(event Custom|Checkpoint%20Activated%20Callback
  (params (CheckID :type Integer) (VehicleNumber :type Integer))
  ;[1 1 1] Tracker Init
  ;;[1 1 1] Checkpoint activation logic
  (bind _checkactivated (CallFunction|ActivateCheck CheckID VehicleNumber))
  (if _checkactivated
    (bind _racerfinished (CallFunction|CheckRacerFinished VehicleNumber))
    (if _racerfinished
      (Default|FinishedRace (Utilities|Array|Get(acopy) (Variables|RacerData|GetVehicles) VehicleNumber))
      (bind _isfinished (CallFunction|CheckRaceFinished))
      (if _isfinished
        (CallFunction|RaceFinished)))))

(event Custom|StartRaceTime
  ;[1 1 1] Race Timer
  (bind _time (Timeline|RaceTimeline Play)
    (:Update
      (bind _output_get (Variables|Default|SetCurrentRaceTime _time))
      (Variables|DisplayText|SetCurrentRaceTimeText (Utilities|TimetoText _output_get)))))

(event Custom|StopRaceTime
  ;[1 1 1] Race Timer
  (bind _time (Timeline|RaceTimeline Stop)
    (:Update
      (bind _output_get (Variables|Default|SetCurrentRaceTime _time))
      (Variables|DisplayText|SetCurrentRaceTimeText (Utilities|TimetoText _output_get)))))

(event Custom|Update%20Positions
  ;[1 1 1] Tracker Init
  ;;[1 1 1] Update the positions of the racers every 1/20th of a second
  (if (and (Utilities|Enum|Equal(Enum) (Variables|Default|GetRaceState) "NewEnumerator1") (Utilities|Enum|Equal(Enum) (Variables|Default|GetTrackerMode) "NewEnumerator1"))
    (CallFunction|AssignPositions false)))

(event EventBeginPlay
  ;[1 1 1] Tracker Init
  (Utilities|FlowControl|Sequence
    (:then_0
      (bind _asracing_game_instance (Utilities|Casting|CastToRacingGameInstance (Game|GetGameInstance)))
      (Variables|Default|SetMaxLaps (Variables|/Game/Blueprints/RacingGameInstance.RacingGameInstance_C|GetLapCount _asracing_game_instance))
      (Variables|Default|SetRaceState "NewEnumerator0")
      ;;[1 1 1] Init vehicle array and racer data
      (for (_array_element _array_index) (Variables|RacerData|GetVehicles)
        (bind _output_get (Variables|/Game/VehicleAdvBP/Blueprints/VehicleBlueprint.VehicleBlueprint_C|SetVehicleNumber _array_element _array_index))
        (Utilities|Array|Add (Variables|RacerData|GetRacers) (Utilities|Struct|MakeRacerData _output_get)))
      ;;[1 1 1] Init HUD
      (CallFunction|InitText)
      (bind _returnvalue (UserInterface|CreateWidget "/Game/Blueprints/UI/RacingHUD.RacingHUD_C"))
      (bind _output_get_2 (Variables|References|SetHUDRef _returnvalue))
      (UserInterface|Viewport|AddtoViewport _output_get_2 0)
      ;;[1 1 1] Allow the tracker to take player input
      (Input|EnableInput (Game|GetPlayerController 0)))
    (:then_1
      ;;[1 1 1] Number each checkpoint
      (for (_array_element_2 _array_index_2) (Variables|CheckpointData|GetCheckpoints)
        (Variables|/Game/Blueprints/Racing/Checkpoint.Checkpoint_C|SetCheckID _array_element_2 _array_index_2)
        (EventDispatchers|BindEventtoCheckpointActivated _array_element_2 (delegate Custom|Checkpoint%20Activated%20Callback)))
      ;;[1 1 1] Set checkcount value
      (Variables|CheckpointData|SetCheckCount (Utilities|Array|Length (Variables|CheckpointData|GetCheckpoints)))
      ;;[1 1 1] Update the positions of the racers every 1/20th of a second
      (bind _returnvalue_2 (Utilities|Time|SetTimerbyEvent (delegate Custom|Update%20Positions) 0.05 true))
      (Variables|Default|SetUpdatePositionsHandle _returnvalue_2))
    (:then_2
      (Default|ShowStartScreen (Variables|References|GetHUDRef)))))

(event Input|ActionEvents|InputActionAccept
  (params (Key :type Key%20Structure :default "None"))
  ;[1 1 1] Accept start action
  (:Pressed
    (switch Utilities|FlowControl|Switch|SwitchonRaceState (Variables|Default|GetRaceState)
      (:NewEnumerator0
        (CallFunction|CountdownStart))
      (:NewEnumerator2
        (Game|OpenLevel(byName) "MainMenu")))))

(fn ConstructionScript)

(fn ActivateCheck
  (params (Checkpoint :type Integer) (RacerID :type Integer))
  ;[1 1 1] Set Local Variables
  (LocalVariables|SetLocalCheckID Checkpoint)
  (LocalVariables|SetLocalRacerID RacerID)
  (LocalVariables|SetLocalRacer (Utilities|Array|Get(acopy) (Variables|RacerData|GetRacers) RacerID))
  ;[1 1 1] If the checkpoint activated is the racers next checkpoint and the racer hasn't finished
  (if (and (== (LocalVariables|GetLocalCheckID) (.NextCheckpoint (Utilities|Struct|BreakRacerData (LocalVariables|GetLocalRacer)))) (not (.Finished (Utilities|Struct|BreakRacerData (LocalVariables|GetLocalRacer)))))
    ;[1 1 1] Increment the racers and lap next checkpoint
    (bind _structout (Utilities|Struct|SetmembersinRacerData (LocalVariables|GetLocalRacer) (Math|Float|Truncate (.Remainder (Math|Float|Division(WholeandRemainder) (Math|Conversions|ToFloat(Integer) (+ (LocalVariables|GetLocalCheckID) 1)) (Math|Conversions|ToFloat(Integer) (Variables|CheckpointData|GetCheckCount))))) (+ (.ReturnValue (Math|Float|Division(WholeandRemainder) (Math|Conversions|ToFloat(Integer) (+ (LocalVariables|GetLocalCheckID) 1)) (Math|Conversions|ToFloat(Integer) (Variables|CheckpointData|GetCheckCount)))) (Utilities|Struct|BreakRacerData (LocalVariables|GetLocalRacer)))))
    (Utilities|Array|SetArrayElem (Variables|RacerData|GetRacers) (LocalVariables|GetLocalRacerID) _structout)
    ;[1 1 1] Update resetloc
    (Variables|/Game/VehicleAdvBP/Blueprints/VehicleBlueprint.VehicleBlueprint_C|SetResetLoc (Utilities|Array|Get(acopy) (Variables|RacerData|GetVehicles) (LocalVariables|GetLocalRacerID)) (Transformation|GetActorTransform (Utilities|Array|Get(acopy) (Variables|CheckpointData|GetCheckpoints) (LocalVariables|GetLocalCheckID))))
    ;[1 1 1] If AI Controlled, update reset node
    (bind _asracing_aicontroller (Utilities|Casting|CastToRacingAIController (Pawn|GetController (Utilities|Array|Get(acopy) (Variables|RacerData|GetVehicles) (LocalVariables|GetLocalRacerID))))
      (:then
        (Default|UpdateResetNode _asracing_aicontroller))
      (:CastFailed
        _))
    ;[1 1 1] If the racer is the displayed racer update the hud
    (if (== (LocalVariables|GetLocalRacerID) (Variables|RacerData|GetDisplayedRacerID))
      (Variables|DisplayText|SetDisplayedRacerLapText (Utilities|Text|ToText(String) (Utilities|String|Append (Utilities|String|ToString(Integer) (.CurrentLap (Utilities|Struct|BreakRacerData (LocalVariables|GetLocalRacer)))) "/" (Utilities|String|ToString(Integer) (Variables|Default|GetMaxLaps))))))
    ;[1 1 1] Debug print info
    (Development|PrintString (Utilities|String|Append "Racer " (Utilities|String|ToString(Integer) (LocalVariables|GetLocalRacerID)) " - Checkpoint " (Utilities|String|ToString(Integer) (+ (LocalVariables|GetLocalCheckID) 1)) "/" (Utilities|String|ToString(Integer) (Variables|CheckpointData|GetCheckCount)) " - Lap " (Utilities|String|ToString(Integer) (.CurrentLap (Utilities|Struct|BreakRacerData (LocalVariables|GetLocalRacer)))) "/" (Utilities|String|ToString(Integer) (Variables|Default|GetMaxLaps))))
    (return true)
    (else
      (return false))))

(fn CheckRacerFinished
  (params (RacerID :type Integer))
  ;[1 1 1] If racer has finished max laps
  (LocalVariables|SetLocalRacer (Utilities|Array|Get(acopy) (Variables|RacerData|GetRacers) RacerID))
  (if (> (.currentlap (LocalVariables|GetLocalRacer)) (Variables|Default|GetMaxLaps))
    ;[1 1 1] Set them to finished and assign their time
    (bind _structout (Utilities|Struct|SetmembersinRacerData (LocalVariables|GetLocalRacer) true (Variables|Default|GetCurrentRaceTime)))
    (Utilities|Array|SetArrayElem (Variables|RacerData|GetRacers) RacerID _structout)
    (return true)
    (else
      (return false))))

(fn CheckRaceFinished
  ;[1 1 1] IsRaceOver is False unless all racers have finished
  (for _array_element (Variables|RacerData|GetRacers)
    (if (not (.Finished (Utilities|Struct|BreakRacerData _array_element)))
      (LocalVariables|SetLocalFinished false)))
  (return (LocalVariables|GetLocalFinished)))

(fn InitText
  (Variables|DisplayText|SetCurrentRaceTimeText (Utilities|TimetoText 0.0))
  (Variables|DisplayText|SetDisplayedRacerLapText (Utilities|Text|ToText(String) (Utilities|String|Append "1/" (Utilities|String|ToString(Integer) (Variables|Default|GetMaxLaps)))))
  (Variables|DisplayText|SetCountdownText "3")
  (Variables|DisplayText|SetDisplayedFinalRaceTime (Utilities|TimetoText 0.0)))

(fn AssignPositions
  (params (Final :type Boolean))
  (bind _localtimes (LocalVariables|GetLocalTimes))
  (bind _checkpoints (Variables|CheckpointData|GetCheckpoints))
  (bind _localdistance (LocalVariables|GetLocalDistance))
  (bind (_indexofmaxvalue _maxvalue) (Math|Float|MaxOfFloatArray _localdistance))
  (bind _indexofminvalue (Math|Float|MinOfFloatArray _localtimes))
  (if Final
    ;[1 1 1] Fill Local Times with the times of all racers
    (for _array_element (Variables|RacerData|GetRacers)
      (Utilities|Array|Add (LocalVariables|GetLocalTimes) (Utilities|Struct|BreakRacerData _array_element)))
    ;[1 1 1] Number the racers by time
    (for _index (range 1 (Utilities|Array|Length (LocalVariables|GetLocalTimes)))
      (bind _structout (Utilities|Struct|SetmembersinRacerData (Utilities|Array|Get(acopy) (Variables|RacerData|GetRacers) _indexofminvalue) _index))
      (Utilities|Array|SetArrayElem (Variables|RacerData|GetRacers) _indexofminvalue _structout)
      (Utilities|Array|SetArrayElem (LocalVariables|GetLocalTimes) _indexofminvalue 999999.0))
    (else
      (Utilities|FlowControl|Sequence
        (:then_0
          ;[1 1 1] Calculate the distance of each racer and store in local distances
          (for _array_element_2 (Variables|RacerData|GetRacers)
            (Utilities|Array|Add (LocalVariables|GetLocalDistance) (+ (Math|Conversions|ToFloat(Integer) (* (Variables|CheckpointData|GetCheckCount) (- (.CurrentLap (Utilities|Struct|BreakRacerData _array_element_2)) 1))) (Math|Conversions|ToFloat(Integer) (Utilities|NegMod (- (.NextCheckpoint (Utilities|Struct|BreakRacerData _array_element_2)) 1) (Variables|CheckpointData|GetCheckCount))) (Math|Float|Min(Float) (/ (Transformation|GetHorizontalDistanceTo (Utilities|Array|Get(acopy) _checkpoints (Utilities|NegMod (- (.NextCheckpoint (Utilities|Struct|BreakRacerData _array_element_2)) 1) (Variables|CheckpointData|GetCheckCount))) (Utilities|Array|Get(acopy) (Variables|RacerData|GetVehicles) (.RacerID (Utilities|Struct|BreakRacerData _array_element_2)))) (Transformation|GetHorizontalDistanceTo (Utilities|Array|Get(acopy) _checkpoints (Utilities|NegMod (- (.NextCheckpoint (Utilities|Struct|BreakRacerData _array_element_2)) 1) (Variables|CheckpointData|GetCheckCount))) (Utilities|Array|Get(acopy) _checkpoints (.NextCheckpoint (Utilities|Struct|BreakRacerData _array_element_2))))) 0.99999)))))
        (:then_1
          ;[1 1 1] Number the racers by distance
          (for _index_2 (range 1 (Utilities|Array|Length (LocalVariables|GetLocalDistance)))
            (bind _structout_2 (Utilities|Struct|SetmembersinRacerData (Utilities|Array|Get(acopy) (Variables|RacerData|GetRacers) _indexofmaxvalue) _index_2 _maxvalue))
            (Utilities|Array|SetArrayElem (Variables|RacerData|GetRacers) _indexofmaxvalue _structout_2)
            (Utilities|Array|SetArrayElem (LocalVariables|GetLocalDistance) _indexofmaxvalue -1.0)))))))