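; Player controller for the racing mode that gates vehicle input according to race state.
; On BeginPlay it caches the controlled vehicle and the Tracker tagged "Master", disables input and binds to the tracker's race start and end events.
; Race start enables input, while race end disables it and zeroes throttle and steering.
; A separate FinishedRace function repeats the same stop logic.
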(event Custom|Race%20End%20Callback
  (bind _vehicleref (Variables|References|GetVehicleRef))
  (bind _vehiclemovement (Variables|/Script/PhysXVehicles.WheeledVehicle|GetVehicleMovement _vehicleref))
  ;[1 1 1] Bind race end event
  (Input|DisableInput _vehicleref self)
  (Class|WheeledVehicleMovementComponent|SetThrottleInput _vehiclemovement 0.0)
  (Class|WheeledVehicleMovementComponent|SetSteeringInput _vehiclemovement 0.0))

(event Custom|RaceStartCallback
  ;[1 1 1] Bind race start event
  (Input|EnableInput (Variables|References|GetVehicleRef) self))

(event EventBeginPlay
  ;[1 1 1] Get Reference to vehicle
  (bind _asvehicle_blueprint (Utilities|Casting|CastToVehicleBlueprint (Pawn|GetControlledPawn)))
  (Variables|References|SetVehicleRef _asvehicle_blueprint)
  ;[1 1 1] Get reference to tracker
  (bind _outactors (Actor|GetAllActorsOfClasswithTag "/Game/Blueprints/Racing/Tracker.Tracker_C" "Master"))
  (bind _astracker (Utilities|Casting|CastToTracker (Utilities|Array|Get(acopy) _outactors)))
  (Variables|References|SetTrackerRef _astracker)
  ;[1 1 1] Disable user input till race is started
  (Input|DisableInput (Variables|References|GetVehicleRef) self)
  ;[1 1 1] Bind race start event
  (EventDispatchers|BindEventtoRaceStart (Variables|References|GetTrackerRef) (delegate Custom|RaceStartCallback))
  ;[1 1 1] Bind race end event
  (EventDispatchers|BindEventtoRaceEnd (Variables|References|GetTrackerRef) (delegate Custom|Race%20End%20Callback)))

(fn ConstructionScript)

(fn FinishedRace
  (bind _vehicleref (Variables|References|GetVehicleRef))
  (bind _vehiclemovement (Variables|/Script/PhysXVehicles.WheeledVehicle|GetVehicleMovement _vehicleref))
  (Input|DisableInput _vehicleref self)
  (Class|WheeledVehicleMovementComponent|SetThrottleInput _vehiclemovement 0.0)
  (Class|WheeledVehicleMovementComponent|SetSteeringInput _vehiclemovement 0.0))