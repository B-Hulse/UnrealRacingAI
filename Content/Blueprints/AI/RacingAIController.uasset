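; AI controller that drives a racing vehicle along AITargetTracker nodes between the Tracker's race start and end events.
; A looping timer sums halving-weight pulls toward upcoming nodes and inverse-square repulsion from nearby cars into steering, with throttle chasing node target speed.
; Rubber-band difficulty updates each second from distance to the player or rival average, scaling look-ahead and speed.
; Cars flipped or slow across a one-second check reset to the saved node.
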(event Custom|Race%20End%20Callback
  (bind _vehicleref (Variables|References|GetVehicleRef))
  (bind _vehiclemovement (Variables|/Script/PhysXVehicles.WheeledVehicle|GetVehicleMovement _vehicleref))
  ;[1 1 1] Bind race end event
  (Class|WheeledVehicleMovementComponent|SetThrottleInput _vehiclemovement 0.0)
  (Class|WheeledVehicleMovementComponent|SetSteeringInput _vehiclemovement 0.0)
  (Utilities|Time|ClearandInvalidateTimerbyHandle (Variables|Default|GetDifficultyUpdateHandle))
  (Utilities|Time|ClearandInvalidateTimerbyHandle (Variables|Default|GetAITickHandle)))

(event Custom|UpdateDifficultyTimerCallback
  ;[1 1 1] Adjust the difficulty once a second
  (if (Variables|Default|GetIsVSPlayer)
    (bind _playerdist (CallFunction|GetPlayerDistance))
    (CallFunction|AdjustDifficulty _playerdist)
    (elif (Variables|Default|GetHasOpponents)
      (bind _averagedist (CallFunction|GetAverageDistance))
      (CallFunction|AdjustDifficulty _averagedist))))

(event Custom|AITick
  ;[1 1 1] Update the AI every 0.05 second (20 times a second)
  (Utilities|FlowControl|Sequence
    (:then_0
      ;;[1 1 1] Car Control
      (bind (_direction _speed) (CallFunction|GetForces))
      (CallFunction|SetDir _direction)
      (CallFunction|SetVel _speed)
      (CallFunction|ControlCar)
      (CallFunction|IncrementNodeCount))
    (:then_1
      ;;[1 1 1] Reset car if flipped for a second
      (bind _stuck (CallFunction|CheckStuck))
      (if _stuck
        (Utilities|FlowControl|Delay 1.0)
        (bind _stuck_2 (CallFunction|CheckStuck))
        (if _stuck_2
          (Default|ResetVehicle (Variables|References|GetVehicleRef))
          (Variables|NodeData|SetCurrNode (Variables|NodeData|GetResetNode)))))))

(event Custom|RaceStartCallback
  ;[1 1 1] Bind race start event
  (bind _returnvalue (Utilities|Time|SetTimerbyEvent (delegate Custom|UpdateDifficultyTimerCallback) 1.0 true))
  (Variables|Default|SetDifficultyUpdateHandle _returnvalue)
  (bind _playeractive (CallFunction|IsAgainstPlayer))
  (Variables|Default|SetIsVSPlayer _playeractive)
  (Variables|Default|SetHasOpponents (> (Utilities|Array|Length (Variables|/Game/Blueprints/Racing/Tracker.Tracker_C|GetRacers (Variables|References|GetTrackerRef))) 1))
  (bind _returnvalue_2 (Utilities|Time|SetTimerbyEvent (delegate Custom|AITick) 0.02 true))
  (Variables|Default|SetAITickHandle _returnvalue_2))

(event EventBeginPlay
  ;[1 1 1] Get Reference to vehicle
  (bind _asvehicle_blueprint (Utilities|Casting|CastToVehicleBlueprint (Pawn|GetControlledPawn)))
  (bind _output_get (Variables|References|SetVehicleRef _asvehicle_blueprint))
  ;[1 1 1] Set vehicle ID
  (Variables|References|SetVehicleID (Variables|/Game/VehicleAdvBP/Blueprints/VehicleBlueprint.VehicleBlueprint_C|GetVehicleNumber _output_get))
  ;[1 1 1] Get reference to tracker
  (bind _outactors (Actor|GetAllActorsOfClasswithTag "/Game/Blueprints/Racing/Tracker.Tracker_C" "Master"))
  (bind _astracker (Utilities|Casting|CastToTracker (Utilities|Array|Get(acopy) _outactors)))
  (Variables|References|SetTrackerRef _astracker)
  ;[1 1 1] Get a reference to the target tracker
  (bind _outactors_2 (Actor|GetAllActorsOfClasswithTag "/Game/Blueprints/AI/AITargetTracker.AITargetTracker_C" "Master"))
  (bind _asaitarget_tracker (Utilities|Casting|CastToAITargetTracker (Utilities|Array|Get(acopy) _outactors_2)))
  (bind _output_get_2 (Variables|References|SetAITrackerRef _asaitarget_tracker))
  ;[1 1 1] Set node count
  (Variables|NodeData|SetNodeCount (Utilities|Array|Length (Variables|/Game/Blueprints/AI/AITargetTracker.AITargetTracker_C|GetNodeArray _output_get_2)))
  ;[1 1 1] Bind race start event
  (EventDispatchers|BindEventtoRaceStart (Variables|References|GetTrackerRef) (delegate Custom|RaceStartCallback))
  ;[1 1 1] Bind race end event
  (EventDispatchers|BindEventtoRaceEnd (Variables|References|GetTrackerRef) (delegate Custom|Race%20End%20Callback)))

(event EventTick
  (params (DeltaSeconds :type Float%20%28single-precision%29)))

(fn ConstructionScript)

(fn GetForces
  (Utilities|FlowControl|Sequence
    (:then_0
      ;[1 1 1] Get node forces
      (for _index (range 0 (Math|Float|Truncate (Variables|Default|GetDifficulty)))
        (LocalVariables|SetLocalForce (+ (* (Math|Vector|Normalize (- (Transformation|GetWorldLocation (Variables|/Game/Blueprints/AI/AITargetNode.AITargetNode_C|GetRoot (Utilities|Array|Get(acopy) (Variables|/Game/Blueprints/AI/AITargetTracker.AITargetTracker_C|GetNodeArray (Variables|References|GetAITrackerRef)) (Math|Integer|%(Integer) (+ _index (Variables|NodeData|GetCurrNode)) (Variables|NodeData|GetNodeCount))))) (Transformation|GetWorldLocation (Variables|/Script/PhysXVehicles.WheeledVehicle|GetMesh (Variables|References|GetVehicleRef))))) (/ 1.0 (Math|Float|Power 2.0 (Math|Conversions|ToFloat(Integer) _index)))) (LocalVariables|GetLocalForce)))))
    (:then_1
      ;[1 1 1] Get vehicle forces
      (for (_array_element _array_index) (Variables|/Game/Blueprints/Racing/Tracker.Tracker_C|GetVehicles (Variables|References|GetTrackerRef))
        (if (!= _array_index (Variables|References|GetVehicleID))
          (if (< (Math|Vector|VectorLength (- (Transformation|GetWorldLocation (Variables|/Script/PhysXVehicles.WheeledVehicle|GetMesh (Variables|References|GetVehicleRef))) (Transformation|GetWorldLocation (Variables|/Script/PhysXVehicles.WheeledVehicle|GetMesh _array_element)))) 2e+02)
            (LocalVariables|SetLocalForce (+ (* (Math|Vector|Normalize (- (Transformation|GetWorldLocation (Variables|/Script/PhysXVehicles.WheeledVehicle|GetMesh (Variables|References|GetVehicleRef))) (Transformation|GetWorldLocation (Variables|/Script/PhysXVehicles.WheeledVehicle|GetMesh _array_element)))) (Math|Float|SafeDivide 4e+03 (Math|Float|Power (Math|Vector|VectorLength (- (Transformation|GetWorldLocation (Variables|/Script/PhysXVehicles.WheeledVehicle|GetMesh (Variables|References|GetVehicleRef))) (Transformation|GetWorldLocation (Variables|/Script/PhysXVehicles.WheeledVehicle|GetMesh _array_element)))) 2.0))) (LocalVariables|GetLocalForce)))))))
    (:then_2
      ;[1 1 1] Return final Vector
      (return (LocalVariables|GetLocalForce) (Variables|/Game/Blueprints/AI/AITargetNode.AITargetNode_C|GetTarget%20Speed (Utilities|Array|Get(acopy) (Variables|/Game/Blueprints/AI/AITargetTracker.AITargetTracker_C|GetNodeArray (Variables|References|GetAITrackerRef)) (Variables|NodeData|GetCurrNode)))))))

(fn SetDir
  (params (Target :type Vector))
  (Variables|Default|SetTargetAngle (Utilities|AngleBetween2DVectors (Math|Conversions|ToVector2D(Vector) Target) (Math|Conversions|ToVector2D(Vector) (Math|Rotator|GetRotationXVector (Transformation|GetWorldRotation (Variables|/Script/PhysXVehicles.WheeledVehicle|GetMesh (Variables|References|GetVehicleRef))))))))

(fn SetVel
  (params (TargetVelIn :type Float%20%28single-precision%29))
  (Variables|Default|SetTargetVel (* TargetVelIn (|(0.700000+(0.100000*Diff)) (Variables|Default|GetDifficulty)))))

(fn ControlCar
  ;[1 1 1] Steer Car
  (Class|WheeledVehicleMovementComponent|SetSteeringInput (Variables|/Script/PhysXVehicles.WheeledVehicle|GetVehicleMovement (Variables|References|GetVehicleRef)) (Math|Float|Clamp(Float) (/ (Variables|Default|GetTargetAngle) 25.0) -1.0))
  ;[1 1 1] Throttle Car
  (Class|WheeledVehicleMovementComponent|SetThrottleInput (Variables|/Script/PhysXVehicles.WheeledVehicle|GetVehicleMovement (Variables|References|GetVehicleRef)) (Math|Float|Clamp(Float) (+ 0.4 (/ (- (Variables|Default|GetTargetVel) (* (Class|WheeledVehicleMovementComponent|GetForwardSpeed (Variables|/Script/PhysXVehicles.WheeledVehicle|GetVehicleMovement (Variables|References|GetVehicleRef))) 0.036)) 5.0)) -1.0)))

(fn IncrementNodeCount
  (if (< (Math|Vector|Distance(Vector) (Transformation|GetWorldLocation (Variables|/Script/PhysXVehicles.WheeledVehicle|GetMesh (Variables|References|GetVehicleRef))) (Transformation|GetWorldLocation (Variables|/Game/Blueprints/AI/AITargetNode.AITargetNode_C|GetRoot (Utilities|Array|Get(acopy) (Variables|/Game/Blueprints/AI/AITargetTracker.AITargetTracker_C|GetNodeArray (Variables|References|GetAITrackerRef)) (Variables|NodeData|GetCurrNode))))) 8e+02)
    (Variables|NodeData|SetCurrNode (Math|Integer|%(Integer) (+ (Variables|NodeData|GetCurrNode) 1) (Variables|NodeData|GetNodeCount)))))

(fn CheckStuck
  (bind _vehicleref (Variables|References|GetVehicleRef))
  (return (or (< (.z (Math|Vector|GetUpVector (Variables|/Script/PhysXVehicles.WheeledVehicle|GetMesh _vehicleref))) 0.0) (< (Class|WheeledVehicleMovementComponent|GetForwardSpeed (Variables|/Script/PhysXVehicles.WheeledVehicle|GetVehicleMovement _vehicleref)) 5e+01))))

(fn GetPlayerDistance
  ;[1 1 1] Store player ID
  (LocalVariables|SetLocalPlayerID (Variables|/Game/Blueprints/Racing/Tracker.Tracker_C|GetDisplayedRacerID (Variables|References|GetTrackerRef)))
  ;[1 1 1] Get player and AI distances
  (LocalVariables|SetLocalAIDist (Utilities|Struct|BreakRacerData (Utilities|Array|Get(acopy) (Variables|/Game/Blueprints/Racing/Tracker.Tracker_C|GetRacers (Variables|References|GetTrackerRef)) (Variables|References|GetVehicleID))))
  (LocalVariables|SetLocalPlayerDist (Utilities|Struct|BreakRacerData (Utilities|Array|Get(acopy) (Variables|/Game/Blueprints/Racing/Tracker.Tracker_C|GetRacers (Variables|References|GetTrackerRef)) (LocalVariables|GetLocalPlayerID))))
  ;[1 1 1] Return the distance from Player to AI
  (bind _output_get (LocalVariables|SetLocalDistDiff (- (LocalVariables|GetLocalAIDist) (LocalVariables|GetLocalPlayerDist))))
  (return _output_get))

(fn AdjustDifficulty
  (params (Distance :type Float%20%28single-precision%29))
  ;[1 1 1] Chage Difficulty by the number of checkpoits ahead/behind the AI is
  (bind _output_get (Variables|Default|SetDifficulty (Math|Float|Clamp(Float) (- (Variables|Default|GetDifficulty) (Math|Float|Clamp(Float) (/ Distance 3.0) -1.5 1.5)) 0.0 3.0)))
  (Development|PrintString (Utilities|String|Append "AI Vehicle:  " (Utilities|String|ToString(Integer) (Variables|References|GetVehicleID)) ", Difficulty: " (Utilities|String|ToString(Float) _output_get))))

(fn IsAgainstPlayer
  ;[1 1 1] Check that a player is controlling a vehicle
  (Utilities|Casting|CastToVehicleBlueprint (Pawn|GetControlledPawn (Game|GetPlayerController 0))
    (:then
      (return true))
    (:CastFailed
      (return false))))

(fn GetAverageDistance
  ;[1 1 1] Find the sum of all AI's (besides the one computing) distances
  (LocalVariables|SetLocalDistSum 0.0)
  (for (_array_element _array_index) (Variables|/Game/Blueprints/Racing/Tracker.Tracker_C|GetRacers (Variables|References|GetTrackerRef))
    (if (!= _array_index (Variables|References|GetVehicleID))
      (LocalVariables|SetLocalDistSum (+ (LocalVariables|GetLocalDistSum) (Utilities|Struct|BreakRacerData _array_element)))
      (else
        (LocalVariables|SetLocalAIDist (Utilities|Struct|BreakRacerData _array_element)))))
  ;[1 1 1] Find the mean distance
  (LocalVariables|SetLocalDistAvg (Math|Float|SafeDivide (LocalVariables|GetLocalDistSum) (Math|Conversions|ToFloat(Integer) (- (Utilities|Array|Length (Variables|/Game/Blueprints/Racing/Tracker.Tracker_C|GetRacers (Variables|References|GetTrackerRef))) 1))))
  ;[1 1 1] Return the distance from the computing AI to the Average Distance
  (bind _output_get (LocalVariables|SetLocalDistDiff (- (LocalVariables|GetLocalAIDist) (LocalVariables|GetLocalDistAvg))))
  (return _output_get))

(fn UpdateResetNode
  (Variables|NodeData|SetResetNode (Variables|NodeData|GetCurrNode)))

(fn FinishedRace
  (bind _vehicleref (Variables|References|GetVehicleRef))
  (bind _vehiclemovement (Variables|/Script/PhysXVehicles.WheeledVehicle|GetVehicleMovement _vehicleref))
  (Class|WheeledVehicleMovementComponent|SetThrottleInput _vehiclemovement 0.0)
  (Class|WheeledVehicleMovementComponent|SetSteeringInput _vehiclemovement 0.0)
  (Utilities|Time|ClearandInvalidateTimerbyHandle (Variables|Default|GetDifficultyUpdateHandle))
  (Utilities|Time|ClearandInvalidateTimerbyHandle (Variables|Default|GetAITickHandle)))