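; SkyCam is a fixed-position racing camera that either tracks a vehicle or free-looks with the mouse.
; On BeginPlay it finds the Master-tagged Tracker and starts locked on its displayed racer, or stays free-look if none exists.
; While locked, Tick aims the camera at the target vehicle, and inputs cycle racers with wraparound.
; Other inputs toggle modes and adjust FOV zoom, while TurnCamera applies free-look with clamped pitch.
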(event EventBeginPlay
  ;[1 1 1] Attempt to get a reference to tracker, else set locked cam to false NOTE: If no tracker exists, free cam only mode is enabled
  (Variables|Default|SetLockedCam false)
  (bind _outactors (Actor|GetAllActorsOfClasswithTag "/Game/Blueprints/Racing/Tracker.Tracker_C" "Master"))
  (if (> (Utilities|Array|Length _outactors) 0)
    (bind _astracker (Utilities|Casting|CastToTracker (Utilities|Array|Get(acopy) _outactors)))
    (bind _output_get (Variables|Default|SetTrackerRef _astracker))
    (Variables|Default|SetTargetVehicleID (Variables|/Game/Blueprints/Racing/Tracker.Tracker_C|GetDisplayedRacerID _output_get))
    (Variables|Default|SetLockedCam true)))

(event EventTick
  (params (DeltaSeconds :type Float%20%28single-precision%29))
  ;[1 1 1] Follow the targeted vehicle if the camera is in follow mode
  (if (Variables|Default|GetLockedCam)
    (Transformation|SetWorldRotation (Variables|Default|GetCamera) (Math|Rotator|FindLookatRotation (Transformation|GetWorldLocation (Variables|Default|GetRoot)) (Transformation|GetWorldLocation (Variables|/Script/PhysXVehicles.WheeledVehicle|GetMesh (Utilities|Array|Get(acopy) (Variables|/Game/Blueprints/Racing/Tracker.Tracker_C|GetVehicles (Variables|Default|GetTrackerRef)) (Variables|Default|GetTargetVehicleID))))) false false)))

(event Input|ActionEvents|InputActionSwitchCamera
  (params (Key :type Key%20Structure))
  ;[1 1 1] Switch the camera between free look and follow mode
  (:Pressed
    (if (Utilities|IsValid (Variables|Default|GetTrackerRef))
      (Variables|Default|SetLockedCam (not (Variables|Default|GetLockedCam))))))

(event Input|ActionEvents|InputActionZoomIn
  (params (Key :type Key%20Structure))
  (bind _camera (Variables|Default|GetCamera))
  ;[1 1 1] Zoom in and out controls
  (:Pressed
    (Camera|SetFieldOfView _camera (- (Variables|/Script/Engine.CameraComponent|GetFieldOfView _camera) (Variables|Default|GetZoom%20Increment)))))

(event Input|ActionEvents|InputActionZoomOut
  (params (Key :type Key%20Structure))
  (bind _camera (Variables|Default|GetCamera))
  ;[1 1 1] Zoom in and out controls
  (:Pressed
    (Camera|SetFieldOfView _camera (+ (Variables|/Script/Engine.CameraComponent|GetFieldOfView _camera) (Variables|Default|GetZoom%20Increment)))))

(event Input|ActionEvents|InputActionSkycamNextRacer
  (params (Key :type Key%20Structure))
  ;[1 1 1] Allow the player to switch the camera focus
  (:Pressed
    (if (Variables|Default|GetLockedCam)
      (Variables|Default|SetTargetVehicleID (Utilities|NegMod (+ (Variables|Default|GetTargetVehicleID) 1) (Utilities|Array|Length (Variables|/Game/Blueprints/Racing/Tracker.Tracker_C|GetRacers (Variables|Default|GetTrackerRef))))))))

(event Input|ActionEvents|InputActionSkycamPrevRacer
  (params (Key :type Key%20Structure))
  ;[1 1 1] Allow the player to switch the camera focus
  (:Pressed
    (if (Variables|Default|GetLockedCam)
      (Variables|Default|SetTargetVehicleID (Utilities|NegMod (- (Variables|Default|GetTargetVehicleID) 1) (Utilities|Array|Length (Variables|/Game/Blueprints/Racing/Tracker.Tracker_C|GetRacers (Variables|Default|GetTrackerRef))))))))

(event Input|AxisEvents|InputAxisLookRight
  (params (AxisValue :type Float%20%28single-precision%29))
  ;[1 1 1] Mouse control for horizontal turning
  (if (not (Variables|Default|GetLockedCam))
    (CallFunction|TurnCamera AxisValue 0.0)))

(event Input|AxisEvents|InputAxisLookUp
  (params (AxisValue :type Float%20%28single-precision%29))
  ;[1 1 1] Mouse control for vertical turning
  (if (not (Variables|Default|GetLockedCam))
    (CallFunction|TurnCamera 0.0 AxisValue)))

(fn ConstructionScript)

(fn TurnCamera
  (params (InYawChange :type Float%20%28single-precision%29) (InPitchChange :type Float%20%28single-precision%29))
  (bind _camera (Variables|Default|GetCamera))
  (bind _returnvalue (Transformation|GetWorldRotation _camera))
  (LocalVariables|SetLocalYaw InYawChange)
  (LocalVariables|SetLocaPitch InPitchChange)
  ;[1 1 1] Apply rotation
  (Transformation|SetWorldRotation (Variables|Default|GetCamera) (Math|Rotator|MakeRotator (.roll _returnvalue) (Math|Float|Clamp(Float) (+ (LocalVariables|GetLocaPitch) (.pitch _returnvalue)) -89.0 89.0) (+ (.yaw _returnvalue) (LocalVariables|GetLocalYaw))) false false))